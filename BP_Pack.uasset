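; BP_Pack is a health pickup actor that restores one point of the player's health on contact.
; The HealthPack component's begin-overlap event casts to BP_Player, adds the health up to a hardcoded cap, then destroys the pack, even at full health.
; If a BP_Projectile overlaps it instead, both the projectile and the pack are destroyed.
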(event `self.HealthPack.OnComponentBeginOverlap`
  (params (OverlappedComponent :type "PrimitiveComponent Object Reference") (OtherActor :type "Actor Object Reference") (OtherComp :type "PrimitiveComponent Object Reference") (OtherBodyIndex :type Integer) (bFromSweep :type Boolean) (SweepResult :type "HitResult Structure (by ref)"))
  (bind _asbp_player (cast `/Game/InfiniteMatrix/Blueprints/BP_Player` OtherActor)
    (:`then`
      (bind _health (`/Game/InfiniteMatrix/Blueprints/BP_Player.Health` _asbp_player))
      (if (< _health 6.0)
        (set `/Game/InfiniteMatrix/Blueprints/BP_Player.Health` (+ _health 1.0) _asbp_player)
        (else
          (set `/Game/InfiniteMatrix/Blueprints/BP_Player.Health` 7.0 _asbp_player)))
      (`self.K2_DestroyActor`))
    (:`CastFailed`
      (bind _asbp_projectile (cast `/Game/InfiniteMatrix/Blueprints/BP_Projectile` OtherActor))
      (`self.K2_DestroyActor` _asbp_projectile)
      (`self.K2_DestroyActor`))))

(fn `UserConstructionScript`)